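; Player character Blueprint for movement along the world X axis, with jumping and wall jumping.
; Jumping while falling triggers WallJump, which line-traces around the capsule and launches the character away from any hit surface.
; Without a hit, WallJump calls itself while JumpCount is at most one, incrementing the count only after that call; landing resets it.
; The construction script sets jump velocity, hold time and the starting count.
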(event `InputAxis|MoveRight`
  (params (AxisValue :type "Float (single-precision)"))
  ;[1 1 1] All Movement Controls
  ;;[1 1 1] Movement
  (`self.AddMovementInput` (1.0 0.0 0.0) AxisValue))

(event `InputAction|Jump`
  (params (Key :type "Key Structure"))
  ;[1 1 1] All Movement Controls
  ;;[1 1 1] Jumping
  (:`Pressed`
    (`self.Jump`)
    (if (`NavMovementComponent.IsFalling` (`self.CharacterMovement`))
      (`self.WallJump`)
      (else
        (set `self.JumpCount` (+ (`self.JumpCount`) 1)))))
  (:`Released`
    (`self.StopJumping`)))

(event `self.OnLanded`
  (params (Hit :type "HitResult Structure (by ref)"))
  ;[1 1 1] All Movement Controls
  ;;[1 1 1] Jumping
  ;;;[1 1 1] Reset JumpCount
  (set `self.JumpCount` 0))

(event `WallJump`
  (bind _returnvalue (`self.GetActorForwardVector`))
  (bind _returnvalue_x (`KismetMathLibrary.BreakVector` (`self.K2_GetActorLocation`)))
  ;[1 1 1] All Movement Controls
  ;;[1 1 1] Jumping
  ;;;[1 1 1] Double and Wall Jump
  (bind (_outhit _returnvalue_2) (`KismetSystemLibrary.LineTraceSingle` (- (`self.K2_GetActorLocation`) (* _returnvalue (+ (`CapsuleComponent.GetScaledCapsuleRadius` (`self.CapsuleComponent`)) 15.0))) (+ (`self.K2_GetActorLocation`) (+ _returnvalue (+ (`CapsuleComponent.GetScaledCapsuleRadius` (`self.CapsuleComponent`)) 15.0))) "TraceTypeQuery1"))
  (if _returnvalue_2
    (`self.LaunchCharacter` (`KismetMathLibrary.MakeVector` (* (`KismetMathLibrary.SignOfFloat` (- _returnvalue_x (.x (`.Location` (`GameplayStatics.BreakHitResult` _outhit))))) 450.0) 0.0 (`CharacterMovementComponent.JumpZVelocity` (`self.CharacterMovement`))) true true)
    (elif (<= (`self.JumpCount`) 1)
      (`self.WallJump`)
      (set `self.JumpCount` (+ (`self.JumpCount`) 1)))))

(fn `UserConstructionScript`
  (set `CharacterMovementComponent.JumpZVelocity` 400.0 (`self.CharacterMovement`))
  (set `self.JumpMaxHoldTime` 0.3)
  (set `self.JumpCount` 0))